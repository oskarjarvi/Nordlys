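; NordlysGameMode is the game mode that spawns and possesses each joining player's character.
; On HandleStartingNewPlayer, the player count picks the PlayerStart by array index and the controller to possess the new pawn.
; The first player gets the Bo third-person character, and every later player gets the Fox character.
; SpawnMPChar is an empty stub.
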(event EventBeginPlay)

(event EventTick
  (params (DeltaSeconds :type Float%20%28single-precision%29)))

(event EventHandleStartingNewPlayer
  (params (NewPlayer :type Player%20Controller%20Object%20Reference))
  (bind _returnvalue (Class|GameModeBase|GetNumPlayers))
  (bind _outactors (Actor|GetAllActorsOfClass "/Script/Engine.PlayerStart"))
  (switch int (- _returnvalue 1)
    (:Default
      (bind _returnvalue_2 (Game|SpawnActorfromClass "/Game/Blueprints/Player/BP_Fox_ThirdPerson1.BP_Fox_ThirdPerson1_C" (Transformation|GetActorTransform (Utilities|Array|Get(acopy) _outactors (- _returnvalue 1))) "Undefined" "MultiplyWithRoot" 0 0))
      (Pawn|Possess (Game|GetPlayerController (- _returnvalue 1)) _returnvalue_2))
    (:0
      (bind _returnvalue_3 (Game|SpawnActorfromClass "/Game/Blueprints/Player/BP_Bo_ThirdPerson.BP_Bo_ThirdPerson_C" (Transformation|GetActorTransform (Utilities|Array|Get(acopy) _outactors (- _returnvalue 1))) "Undefined" "MultiplyWithRoot" 0 0))
      (Pawn|Possess (Game|GetPlayerController (- _returnvalue 1)) _returnvalue_3))))

(fn ConstructionScript)

(fn SpawnMPChar
  (params (Player%20Controller%20Ref :type Controller%20Object%20Reference)))